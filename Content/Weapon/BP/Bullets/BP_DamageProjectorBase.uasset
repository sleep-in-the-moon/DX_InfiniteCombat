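; BP_DamageProjectorBase is a weapon bullet base Blueprint that deals damage through the Gameplay Ability System.
; On BeginPlay it binds HitEvent to the DGProjector hit callback.
; When both hit actor and owner have an ICAbilitySystemComponent, the owner's component applies GE_DamageApply to the target, passing a HitDamage-derived magnitude via the SetByCaller.Damage tag.
; Direct GE_DamageApply and GE_AddHitTag applications remain as unconnected nodes.
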(event `self.ReceiveBeginPlay`
  (add `self.DG_ProjectorHitObj` (delegate `HitEvent`)))

(event `HitEvent` :!signature `self.DG_ProjectorHitObj`
  (params (HitRes :type "HitResult Structure"))
  (bind _returnvalue (`self.GetComponentByClass` HitRes_HitActor "/Script/DX_InfiniteCombat.ICAbilitySystemComponent"))
  (bind _returnvalue_2 (`self.GetComponentByClass` (`self.GetOwner`) "/Script/DX_InfiniteCombat.ICAbilitySystemComponent"))
  (`/Engine/EditorBlueprintResources/StandardMacros.IsValid` _returnvalue
    (:`Is Valid`
      (`/Engine/EditorBlueprintResources/StandardMacros.IsValid` _returnvalue_2
        (:`Is Valid`
          (bind _output_get (set `self.Hit Damage` (`self.HitDamage`)))
          (bind _result (`/Engine/EditorBlueprintResources/StandardMacros.NegateFloat` _output_get)
            (:`  `
              (`ICAbilitySystemComponent.ApplySetByCallerGEToTarget` _returnvalue_2 _returnvalue "/Game/Character/GAS/GE/GE_DamageApply.GE_DamageApply_C" (struct :`TagName` "SetByCaller.Damage") _result 0.0))))))))

(fn `UserConstructionScript`)