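; BP_PC_Main is a player controller Blueprint that sets up the player's main state HUD.
; On BeginPlay it creates WBP_MainState for itself, adds it to the player screen and stores it as CombatStatesWidget.
; Tick only calls the parent, and a debug arrow showing move input from the player character is left unconnected, so it never runs.
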(event `self.ReceiveBeginPlay`
  (`parent.ReceiveBeginPlay`)
  (bind _returnvalue (`|CreateWidget` "/Game/Widgets/WBP/WBP_MainState.WBP_MainState_C" self))
  (`UserWidget.AddToPlayerScreen` _returnvalue 0)
  (set `self.CombatStatesWidget` _returnvalue))

(event `self.ReceiveTick`
  (params (DeltaSeconds :type "Float (single-precision)"))
  (`parent.ReceiveTick` DeltaSeconds))

(fn `UserConstructionScript`)