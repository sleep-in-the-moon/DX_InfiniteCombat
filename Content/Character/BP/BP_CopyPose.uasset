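; BP_CopyPose is a short-lived actor that shows a frozen copy of a character's pose, with a helmet on the head.
; The construction script adds a collision-free helmet static mesh and snaps it to the head socket of a PoseableMesh.
; On BeginPlay, the PoseableMesh copies the pose once from a supplied skeletal component, then the actor destroys itself after a configurable delay.
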(event `self.ReceiveBeginPlay`
  (`PoseableMeshComponent.CopyPoseFromSkeletalComponent` (`self.PoseableMesh`) (`self.In Component to Copy`))
  (`KismetSystemLibrary.Delay` (`self.DestoryTime`))
  (`self.K2_DestroyActor`))

(fn `UserConstructionScript`
  (bind _returnvalue (`AddComponent|NODE_AddStaticMeshComponent-0`))
  (`SceneComponent.K2_AttachToComponent` _returnvalue (`self.PoseableMesh`) "Head_Socket" "SnapToTarget" "SnapToTarget" "KeepRelative" false)
  (`StaticMeshComponent.SetStaticMesh` _returnvalue "/Game/Character/Assets/Samurai2/Meshes/SM_Helmet_1.SM_Helmet_1")
  (`PrimitiveComponent.SetCollisionEnabled` _returnvalue "NoCollision"))