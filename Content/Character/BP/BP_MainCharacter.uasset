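; Player character Blueprint for a Gameplay Ability System combat game with katana and bow weapons.
; BeginPlay attaches head and sheath meshes to sockets, equips the katana through GA_SwitchWeapon_BP and forwards health changes to the controller's HUD widget.
; The ASC immunity callback plays a sound, spawns a pose-copy afterimage and briefly applies slow motion with color dispersion.
; Debug keys drive sprint, weapon switching, debug display, custom movement mode and time dilation.
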(event ImmunityGECallback(ASC)
  (params (ImmunityGETags :type Gameplay%20Tag%20Container%20Structure%20%28by%20ref%29))
  (bind _mesh (Variables|Character|GetMesh))
  (Audio|PlaySound2D "/Engine/EditorSounds/GamePreview/StartSimulate.StartSimulate" 1.0 1.0 0.0 0 0)
  (Game|SpawnActorfromClass "/Game/Character/BP/BP_CopyPose.BP_CopyPose_C" (Transformation|GetWorldTransform _mesh) "Undefined" "MultiplyWithRoot" 0 _mesh 0.8 0)
  (Utilities|Time|SetGlobalTimeDilation 0.5)
  (Rendering|Material|SetScalarParameterValue (Variables|Default|GetMPC_Post) (Utilities|Name|MakeLiteralName "EnableColorDispersion") 1.0 :!class /Script/Engine.KismetMaterialLibrary)
  (Utilities|FlowControl|Delay 0.4)
  (Utilities|Time|SetGlobalTimeDilation 1.0)
  (Rendering|Material|SetScalarParameterValue (Variables|Default|GetMPC_Post) (Utilities|Name|MakeLiteralName "EnableColorDispersion") 0.0 :!class /Script/Engine.KismetMaterialLibrary))

(event Custom|HelthChange
  (params (NewHelth :type Float%20%28single-precision%29))
  (bind _asc (Variables|Default|GetASC))
  (bind (_bsuccessfullyfoundattribute _returnvalue) (Ability|Attribute|GetFloatAttributefromAbilitySystemComponent _asc "(AttributeName=\"MaxHP\",Attribute=/Script/DX_InfiniteCombat.CharacterAttributeSet:MaxHP,AttributeOwner=\"/Script/CoreUObject.Class'/Script/DX_InfiniteCombat.CharacterAttributeSet'\")"))
  (if _bsuccessfullyfoundattribute
    (bind _asbp_pc_main (Utilities|Casting|CastToBP_PC_Main (Pawn|GetController)))
    (Default|UpdateHelth (Variables|/Game/Main/Gameplay/BP_PC_Main.BP_PC_Main_C|GetCombatStatesWidget _asbp_pc_main) (/ NewHelth _returnvalue))))

(event Input|EnhancedActionEvents|EnhancedInputActionIA_UIMenu
  (params (ActionValue :type Boolean) (ElapsedSeconds :type Float%20%28double-precision%29) (TriggeredSeconds :type Float%20%28double-precision%29) (InputAction :type Input%20Action%20Object%20Reference :default "/Game/Main/Input/IA_UIMenu.IA_UIMenu"))
  (:Completed
    (bind _asbp_pc_main (Utilities|Casting|CastToBP_PC_Main (Pawn|GetController)))
    (Default|TriggerUIMenu _asbp_pc_main)))

(event EventBeginPlay
  (|CallParentFunction)
  (Utilities|FlowControl|Sequence
    (:then_0
      (CallFunction|AddStaticMeshtoSocket "/Game/Character/Assets/Samurai2/Meshes/SamuraiHead.SamuraiHead" "Head_Socket" (Math|Transform|MakeTransform "0.000000,3.000000,-5.000000" "0.000000,0.000000,7.000000" "0.070000,0.070000,0.070000") true)
      (CallFunction|AddStaticMeshtoSocket :StaticMesh "/Game/Character/Assets/Samurai2/Meshes/SM_Sheath_2.SM_Sheath_2" :SocketName "Belt_Socket")
      (bind _returnvalue (Utilities|InstancedStruct|MakeInstancedStruct (GameplayTags|MakeLiteralGameplayTag "(TagName=\"Weapon.Katana\")")))
      (Class|ICAbilitySystemComponent|TryActivateAbilitybyClassArg (Variables|Default|GetASC) "/Game/Character/GAS/GA/GA_SwitchWeapon_BP.GA_SwitchWeapon_BP_C" _returnvalue true))
    (:then_1
      (EventDispatchers|BindEventtoHelthChangeBPDG (Variables|Default|GetASC) (delegate Custom|HelthChange)))))

(event Input|KeyboardEvents|DebugKey3
  (params (Key :type Key%20Structure :default "None") (ActionValue :type Input%20Action%20Value%20Structure))
  ;[0.15 0.15 0.15 0.5] Debug
  (:Pressed
    (bind _isa (Utilities|FlowControl|FlipFlop)
      (:A
        _)
      (:B
        _))
    (Class|ICWorldSubsystem|SetShowDebug (Subsystems|GetICWorldSubsystem) _isa)))

(event Input|KeyboardEvents|DebugKey2
  (params (Key :type Key%20Structure :default "None") (ActionValue :type Input%20Action%20Value%20Structure))
  ;[0.15 0.15 0.15 0.5] Debug
  (:Pressed
    (bind _returnvalue (Utilities|InstancedStruct|MakeInstancedStruct (GameplayTags|MakeLiteralGameplayTag "(TagName=\"Weapon.Bow\")")))
    (Class|ICAbilitySystemComponent|TryActivateAbilitybyClassArg (Variables|Default|GetASC) "/Game/Character/GAS/GA/GA_SwitchWeapon_BP.GA_SwitchWeapon_BP_C" _returnvalue true)))

(event Input|KeyboardEvents|DebugKey1
  (params (Key :type Key%20Structure :default "None") (ActionValue :type Input%20Action%20Value%20Structure))
  ;[0.15 0.15 0.15 0.5] Debug
  (:Pressed
    (bind _returnvalue (Utilities|InstancedStruct|MakeInstancedStruct (GameplayTags|MakeLiteralGameplayTag "(TagName=\"Weapon.Katana\")")))
    (Class|ICAbilitySystemComponent|TryActivateAbilitybyClassArg (Variables|Default|GetASC) "/Game/Character/GAS/GA/GA_SwitchWeapon_BP.GA_SwitchWeapon_BP_C" _returnvalue true)))

(event Input|KeyboardEvents|DebugKeyZ
  (params (Key :type Key%20Structure :default "None") (ActionValue :type Input%20Action%20Value%20Structure))
  ;[0.15 0.15 0.15 0.5] Debug
  (:Pressed
    (Utilities|FlowControl|FlipFlop
      (:A
        (Utilities|Time|SetGlobalTimeDilation 0.25))
      (:B
        (Utilities|Time|SetGlobalTimeDilation 1.0)))))

(event Input|KeyboardEvents|DebugKey6
  (params (Key :type Key%20Structure :default "None") (ActionValue :type Input%20Action%20Value%20Structure))
  (bind _charactermovement (Variables|Character|GetCharacterMovement))
  ;[0.15 0.15 0.15 0.5] Debug
  (:Pressed
    (Pawn|Components|CharacterMovement|SetMovementMode _charactermovement "MOVE_Custom" 1)
    (Variables|/Script/Engine.CharacterMovementComponent|SetbOrientRotationToMovement (Variables|Character|GetCharacterMovement) false)
    (Development|PrintString (Utilities|String|EnumtoString (Variables|/Script/Engine.CharacterMovementComponent|GetMovementMode _charactermovement)))))

(event Input|KeyboardEvents|DebugKey7
  (params (Key :type Key%20Structure :default "None") (ActionValue :type Input%20Action%20Value%20Structure))
  (bind _charactermovement (Variables|Character|GetCharacterMovement))
  ;[0.15 0.15 0.15 0.5] Debug
  (:Pressed
    (Pawn|Components|CharacterMovement|SetMovementMode _charactermovement "MOVE_Walking" 0)
    (Variables|/Script/Engine.CharacterMovementComponent|SetbOrientRotationToMovement (Variables|Character|GetCharacterMovement) true)
    (Development|PrintString (Utilities|String|EnumtoString (Variables|/Script/Engine.CharacterMovementComponent|GetMovementMode _charactermovement)))))

(event Input|KeyboardEvents|LeftShift
  (params (Key :type Key%20Structure :default "None"))
  (bind _charactermovement (Variables|Character|GetCharacterMovement))
  ;[0.15 0.15 0.15 0.5] Debug
  (:Pressed
    (Variables|/Script/Engine.CharacterMovementComponent|SetMaxWalkSpeed _charactermovement 1e+03))
  (:Released
    (Variables|/Script/Engine.CharacterMovementComponent|SetMaxWalkSpeed _charactermovement 6e+02)))

(fn ConstructionScript)

(fn AddStaticMeshtoSocket
  (params (StaticMesh :type Static%20Mesh%20Object%20Reference) (SocketName :type Name) (RelativeTrans :type Transform) (HaveRelativeTrans :type Boolean))
  (bind (_location _rotation _scale) (Math|Transform|BreakTransform RelativeTrans))
  (bind _returnvalue (AddComponent|AddStaticMeshComponent false))
  (bind _returnvalue_2 (Components|StaticMesh|SetStaticMesh _returnvalue StaticMesh))
  (if _returnvalue_2
    (Collision|SetCollisionEnabled _returnvalue "NoCollision")
    (bind _returnvalue_3 (Transformation|AttachComponentToComponent _returnvalue (Variables|Character|GetMesh) SocketName "KeepRelative" "KeepRelative" "KeepRelative" false))
    (if (and HaveRelativeTrans _returnvalue_3)
      (Transformation|SetRelativeTransform _returnvalue (Math|Transform|MakeTransform _location _rotation _scale) false false))))

(fn GetModuleName
  (return "ComboConfig"))