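; GAS attack ability that branches on the owner's weapon tag, falling back to the current weapon's AttackGATriggerTag ability.
; Katana plays an air attack or a charge with UI bar, releasing into the current combo section or, when fully charged, a dash attack.
; Bow draws while input is held and launches an arrow with the held time unless dodging.
; Ending restores move input and advances the combo through MontageComboMap or resets it.
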(event `self.K2_ActivateAbility`
  (bind _returnvalue (`self.GetOwningActorFromActorInfo`))
  (bind _returnvalue_2 (`BlueprintGameplayTagLibrary.MakeLiteralGameplayTagContainer` (struct :`GameplayTags` (struct :`(TagName` "State.InCharge.AttackCharge")))))
  (bind _returnvalue_3 (`self.GetAbilitySystemComponentFromActorInfo`))
  (bind _returnvalue_4 (`self.GetOwningActorFromActorInfo`))
  (bind _returnvalue_5 (`self.GetOwningActorFromActorInfo`))
  (bind _returnvalue_6 (`self.GetOwningActorFromActorInfo`))
  (bind _returnvalue_7 (`BlueprintGameplayTagLibrary.MakeLiteralGameplayTagContainer` (struct :`GameplayTags` (struct :`(TagName` "State.InCharge.AttackCharge")))))
  (bind _returnvalue_8 (`self.GetOwningActorFromActorInfo`))
  (bind _returnvalue_9 (`Actor.GetComponentByClass` (`self.GetOwningActorFromActorInfo`) "/Script/DX_InfiniteCombat.CombatCharacterComponent"))
  (bind ((`AttackGATriggerTag` _attackgatriggertag)) (break `WeaponStruct` (`CombatCharacterComponent.GetCurWeapon` _returnvalue_9)))
  (bind _returnvalue_10 (`self.K2_CommitAbility`))
  (if _returnvalue_10
    (bind _asicability_system_component (cast `ICAbilitySystemComponent` _returnvalue_3))
    (`|SwitchGameplayTag` (`ICAbilitySystemComponent.GetFirstChildTag` _asicability_system_component (struct :`TagName` "Weapon"))
      (:`Default`
        (`/Engine/EditorBlueprintResources/StandardMacros.IsValid` _returnvalue_9
          (:`Is Valid`
            (if (`BlueprintGameplayTagLibrary.IsGameplayTagValid` _attackgatriggertag)
              (`AbilitySystemComponent.TryActivateAbilitiesByTag` _returnvalue_3 (`BlueprintGameplayTagLibrary.MakeGameplayTagContainerFromTag` _attackgatriggertag) true)))))
      (:`Weapon.Katana`
        (if (`GameplayTagAssetInterface.HasMatchingGameplayTag` _returnvalue_3 (struct :`TagName` "State.InAir"))
          (`Controller.SetIgnoreMoveInput` (`GameplayStatics.GetPlayerController` 0) true)
          (`AbilityTask_PlayMontageAndWait.CreatePlayMontageAndWaitProxy` "None" "/Game/Character/Assets/Samurai2/ReTargetAnim/Anim/Montage/AM_AirAttackUnsheath.AM_AirAttackUnsheath"
            (:`OnCompleted`
              _)
            (:`OnInterrupted`
              _)
            (:`OnCancelled`
              _))
          (set `self.RestartCombo` true)
          (`self.K2_EndAbility`)
          (else
            (`Controller.SetIgnoreMoveInput` (`GameplayStatics.GetPlayerController` 0) true)
            (bind _aspawn (cast `Pawn` (`self.GetOwningActorFromActorInfo`)))
            (`AbilitySystemBlueprintLibrary.AddLooseGameplayTags` _returnvalue_6 _returnvalue_7 true)
            (`AbilitySystemBlueprintLibrary.RemoveLooseGameplayTags` _returnvalue_6 (`BlueprintGameplayTagLibrary.MakeLiteralGameplayTagContainer` (struct :`GameplayTags` (struct :`(TagName` "State.InCombo")))) true)
            (`AbilityTask_PlayMontageAndWait.CreatePlayMontageAndWaitProxy` "None" "/Game/Character/Assets/Samurai2/ReTargetAnim/Anim/Attack/AM_Charge.AM_Charge" 1.0 "None" true 1.0 0.0 true
              (:`then`
                (bind _returnvalue_11 (`|CreateWidget` "/Game/Widgets/WBP_ChargeBar.WBP_ChargeBar_C"))
                (bind _output_get (set `self.ChargeUI` _returnvalue_11))
                (`UserWidget.AddToViewport` _returnvalue_11 0)
                (`UserWidget.AddToViewport` _output_get 0)
                (`/Game/Widgets/WBP_ChargeBar.SetChargeTime` _output_get (`self.ChargeTime`))
                (bind (_asynctaskproxy _heldtime) (`AbilityTask_ICWaitInputReleased.ICWaitInputReleased` 0.2)
                  (:`OnReleased`
                    (`|ExecutionSequence`
                      (:`then_0`
                        (`AbilitySystemBlueprintLibrary.AddLooseGameplayTags` _returnvalue_8 (`BlueprintGameplayTagLibrary.MakeLiteralGameplayTagContainer` (struct :`GameplayTags` (struct :`(TagName` "State.InCombo")))) true)
                        (`self.MontageStop` -1.0)
                        (`AbilitySystemBlueprintLibrary.RemoveLooseGameplayTags` _returnvalue_8 _returnvalue_7 true)
                        (if (< _heldtime (`self.ChargeTime`))
                          (`AbilityTask_PlayMontageAndWait.CreatePlayMontageAndWaitProxy` "None" "/Game/Character/Assets/Samurai2/ReTargetAnim/Anim/Montage/Combo1_Attack1_Root_Montage.Combo1_Attack1_Root_Montage" 1.0 (`self.CurrentComboSection`) true 1.0 0.0 true
                            (:`OnCompleted`
                              (set `self.RestartCombo` true :!label _label)
                              (`self.K2_EndAbility`))
                            (:`OnInterrupted`
                              (`self.K2_EndAbility` :!label _label_2))
                            (:`OnCancelled`
                              (goto _label)))
                          (else
                            (`AbilityTask_PlayMontageAndWait.CreatePlayMontageAndWaitProxy` "None" "/Game/Character/Assets/Samurai2/ReTargetAnim/Anim/Attack/AS_Dash_Air_Attack_Seq_Montage.AS_Dash_Air_Attack_Seq_Montage" 1.0 "None" true 1.0 0.0 true
                              (:`OnCompleted`
                                (goto _label))
                              (:`OnInterrupted`
                                (goto _label_2))
                              (:`OnCancelled`
                                (goto _label))))))
                      (:`then_1`
                        (`/Game/Widgets/WBP_ChargeBar.ChangeIncrement` _output_get false)
                        (`GameplayTask_WaitDelay.TaskWaitDelay` null 0.5
                          (:`OnFinish`
                            (`Widget.RemoveFromParent` _output_get))))))))))))
      (:`Weapon.Bow`
        (if (`KismetSystemLibrary.DoesImplementInterface` _returnvalue_4 "/Game/Character/Interface/BPI_BowCharacter.BPI_BowCharacter_C")
          (if (not (`GameplayTagAssetInterface.HasMatchingGameplayTag` (`self.GetAbilitySystemComponentFromActorInfo`) (struct :`TagName` "Weapon.Bow.Arrow")))
            (message `/Game/Character/Interface/BPI_BowCharacter.PrepareArrow` _returnvalue_4))
          (message `/Game/Character/Interface/BPI_BowCharacter.InBowState` _returnvalue_4)
          (`AbilitySystemBlueprintLibrary.AddLooseGameplayTags` _returnvalue_5 _returnvalue_2 true)
          (bind (_asynctaskproxy_2 _heldtime_2) (`AbilityTask_ICWaitInputReleased.ICWaitInputReleased` 0.2)
            (:`then`
              ; 待机-》拉弓
              (`AbilityTask_PlayMontageAndWait.CreatePlayMontageAndWaitProxy` "None" "/Game/Character/Assets/Samurai2/ReTargetAnim/Anim/Bow/Montage/Anim_BOW_aim_ST_FWD_Montage.Anim_BOW_aim_ST_FWD_Montage"))
            (:`OnReleased`
              (`AbilitySystemBlueprintLibrary.RemoveLooseGameplayTags` _returnvalue_5 _returnvalue_2 true)
              (if (`GameplayTagAssetInterface.HasMatchingGameplayTag` (`self.GetAbilitySystemComponentFromActorInfo`) (struct :`TagName` "State.InDodge"))
                (`self.K2_EndAbility`)
                (else
                  (message `/Game/Character/Interface/BPI_BowCharacter.OutBowState` _returnvalue)
                  (`self.MontageStop` -1.0)
                  (message `/Game/Character/Interface/BPI_BowCharacter.LaunchArrow` _returnvalue _heldtime_2)
                  (`self.K2_EndAbility`))))))))))

(event `self.K2_OnEndAbility`
  (params (bWasCancelled :type Boolean))
  (bind (_value _returnvalue) (`BlueprintMapLibrary.Map_Find` (`self.MontageComboMap`) (`self.CurrentComboSection`)))
  (`Controller.SetIgnoreMoveInput` (`GameplayStatics.GetPlayerController` 0) false)
  (`AbilitySystemBlueprintLibrary.RemoveLooseGameplayTags` (`self.GetOwningActorFromActorInfo`) (`BlueprintGameplayTagLibrary.MakeLiteralGameplayTagContainer` (struct :`GameplayTags` (struct :`(TagName` "State.LockAttack") :`(TagName` "State.InCombo")))))
  (if (`self.RestartCombo`)
    (set `self.CurrentComboSection` "FirstCombo")
    (elif _returnvalue
      (set `self.CurrentComboSection` (break `ComboInfo` _value))
      (else
        (set `self.CurrentComboSection` "FirstCombo"))))
  (`self.ResetValue`))

(fn `ResetValue`
  (bind _chargeui (`self.ChargeUI`))
  (set `self.RestartCombo` false)
  (`/Engine/EditorBlueprintResources/StandardMacros.IsValid` _chargeui
    (:`Is Valid`
      (`Widget.RemoveFromParent` _chargeui))))