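; Gameplay ability for a staff attack that fires a magic bullet at player character 0, apparently for AI combatants.
; After commit, it checks for a Staff weapon, holds it and plays its linked montage.
; On blend out, or immediately without a montage, it spawns BP_MagicBullet at the weapon socket, launches it with placeholder parameters, enables socket tracing and passes the player to TraceObj.
; It clears State.LockAttack on firing, completion or interruption; EndAbility is never called.
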(event `self.K2_ActivateAbility`
  (bind _returnvalue (`self.GetOwningActorFromActorInfo`))
  (bind _returnvalue_2 (`GameplayStatics.GetPlayerCharacter` 0))
  (bind _returnvalue_3 (`Actor.GetComponentByClass` (`self.GetOwningActorFromActorInfo`) "/Script/DX_InfiniteCombat.CombatCharacterComponent"))
  (bind ((`WeaponTag` _weapontag) (`TagLinkMontage` _taglinkmontage)) (break `WeaponStruct` (`CombatCharacterComponent.GetCurWeapon` _returnvalue_3)))
  (bind _returnvalue_4 (`SceneComponent.GetSocketLocation` (`CombatCharacterComponent.GetWeaponComponent` _returnvalue_3) "BulletLaunchLoc"))
  (bind (_value _returnvalue_5) (`BlueprintMapLibrary.Map_Find` _taglinkmontage (struct :`TagName` "Weapon.Staff")))
  (bind _returnvalue_6 (`self.K2_CommitAbility`))
  (if _returnvalue_6
    (`/Engine/EditorBlueprintResources/StandardMacros.IsValid` _returnvalue_3
      (:`Is Valid`
        (if (== _weapontag (struct :`TagName` "Weapon.Staff"))
          (`CombatCharacterComponent.WeaponToHeld` _returnvalue_3)
          (if _returnvalue_5
            (`AbilityTask_PlayMontageAndWait.CreatePlayMontageAndWaitProxy` "None" _value
              (:`OnCompleted`
                (`AbilitySystemBlueprintLibrary.RemoveLooseGameplayTags` _returnvalue (`BlueprintGameplayTagLibrary.MakeLiteralGameplayTagContainer` (struct :`GameplayTags` (struct :`(TagName` "State.LockAttack")))) :!label _label))
              (:`OnBlendOut`
                (bind _returnvalue_7 (`|SpawnActorFromClass` "/Game/Weapon/BP/Bullets/BP_MagicBullet.BP_MagicBullet_C" (`KismetMathLibrary.MakeTransform` _returnvalue_4) "Undefined" "MultiplyWithRoot" _returnvalue null :!label _label_2))
                (`AbilitySystemBlueprintLibrary.RemoveLooseGameplayTags` _returnvalue (`BlueprintGameplayTagLibrary.MakeLiteralGameplayTagContainer` (struct :`GameplayTags` (struct :`(TagName` "State.LockAttack")))))
                (`ProjectorActorBase.Launch` _returnvalue_7 0.0 (`KismetMathLibrary.Normal` (- (`Actor.K2_GetActorLocation` _returnvalue_2) _returnvalue_4)) 10.0)
                (`ProjectorActorBase.EnableTraceBySocketName` _returnvalue_7 (`|MakeArray` "ObjectTypeQuery1" "ObjectTypeQuery3" :!type "EObjectTypeQuery Enum") true "DamageLoc")
                (`ProjectorActorBase.TraceObj` _returnvalue_7 _returnvalue_2))
              (:`OnInterrupted`
                (goto _label))
              (:`OnCancelled`
                (goto _label)))
            (else
              (goto _label_2))))))))