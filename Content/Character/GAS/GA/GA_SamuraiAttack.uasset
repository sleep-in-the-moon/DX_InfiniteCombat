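; Samurai attack gameplay ability that tries a WeakLock trace, then branches on the current weapon tag, forwarding unhandled tags to abilities matching that tag.
; Katana plays an air attack when airborne; grounded, it shows a charge bar and release timing selects a combo montage or charged dash attack.
; Bow aims while held and launches an arrow using held time on release, unless dodging.
; Ability end advances the combo section through MontageComboMap or resets it.
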(event `self.K2_ActivateAbility`
  (bind _returnvalue (`BlueprintGameplayTagLibrary.MakeLiteralGameplayTagContainer` (struct :`GameplayTags` (struct :`(TagName` "State.InCharge.AttackCharge")))))
  (bind _returnvalue_2 (`self.GetAbilitySystemComponentFromActorInfo`))
  (bind _returnvalue_3 (`self.GetOwningActorFromActorInfo`))
  (bind _returnvalue_4 (`self.GetOwningActorFromActorInfo`))
  (bind _returnvalue_5 (`BlueprintGameplayTagLibrary.MakeLiteralGameplayTagContainer` (struct :`GameplayTags` (struct :`(TagName` "State.InCharge.AttackCharge")))))
  (bind _returnvalue_6 (`self.GetOwningActorFromActorInfo`))
  (bind _returnvalue_7 (`Actor.GetComponentByClass` (`self.GetAvatarActorFromActorInfo`) "/Script/DX_InfiniteCombat.CombatCharacterComponent"))
  (bind _returnvalue_8 (`Actor.GetComponentByClass` (`self.GetAvatarActorFromActorInfo`) "/Script/DX_InfiniteCombat.BowComponent"))
  (bind _returnvalue_9 (`Actor.GetComponentByClass` (`self.GetAvatarActorFromActorInfo`) "/Script/DX_InfiniteCombat.WeakLockComponent"))
  (bind _weapontag (`WeaponDataAsset.WeaponTag` (`CombatCharacterComponent.GetCurrentWeapon` _returnvalue_7)))
  (bind _returnvalue_10 (`self.K2_CommitAbility`))
  (if _returnvalue_10
    (`/Engine/EditorBlueprintResources/StandardMacros.IsValid` _returnvalue_9
      (:`Is Valid`
        (`WeakLockComponent.TryLockByTrace` _returnvalue_9))
      (:`Is Not Valid`
        _))
    (`|SwitchGameplayTag` _weapontag
      (:`Default`
        (`/Engine/EditorBlueprintResources/StandardMacros.IsValid` _returnvalue_7
          (:`Is Valid`
            (if (`BlueprintGameplayTagLibrary.IsGameplayTagValid` _weapontag)
              (`AbilitySystemComponent.TryActivateAbilitiesByTag` _returnvalue_2 (`BlueprintGameplayTagLibrary.MakeGameplayTagContainerFromTag` _weapontag) true)))))
      (:`Weapon.Katana`
        (if (`GameplayTagAssetInterface.HasMatchingGameplayTag` _returnvalue_2 (struct :`TagName` "State.InAir"))
          (`Controller.SetIgnoreMoveInput` (`GameplayStatics.GetPlayerController` 0) true)
          (`AbilityTask_PlayMontageAndWait.CreatePlayMontageAndWaitProxy` "None" "/Game/Character/Assets/Samurai2/ReTargetAnim/Anim/Attack/Montage/AM_AirAttackUnsheath.AM_AirAttackUnsheath"
            (:`OnCompleted`
              _)
            (:`OnInterrupted`
              _)
            (:`OnCancelled`
              _))
          (set `self.RestartCombo` true)
          (`self.K2_EndAbility`)
          (else
            (`Controller.SetIgnoreMoveInput` (`GameplayStatics.GetPlayerController` 0) true)
            (bind _aspawn (cast `Pawn` (`self.GetAvatarActorFromActorInfo`)))
            (`AbilitySystemBlueprintLibrary.AddLooseGameplayTags` _returnvalue_4 _returnvalue_5 true)
            (`AbilitySystemBlueprintLibrary.RemoveLooseGameplayTags` _returnvalue_4 (`BlueprintGameplayTagLibrary.MakeLiteralGameplayTagContainer` (struct :`GameplayTags` (struct :`(TagName` "State.InCombo")))) true)
            (`AbilityTask_PlayMontageAndWait.CreatePlayMontageAndWaitProxy` "None" "/Game/Character/Assets/Samurai2/ReTargetAnim/Anim/Attack/Montage/AM_Charge.AM_Charge" 1.0 "None" true 1.0 0.0 true
              (:`then`
                (bind _returnvalue_11 (`|CreateWidget` "/Game/Widgets/WBP/WBP_ChargeBar.WBP_ChargeBar_C"))
                (bind _output_get (set `self.WBPCharge` _returnvalue_11))
                (`UserWidget.AddToViewport` _output_get 0)
                (`/Game/Widgets/WBP/WBP_ChargeBar.SetChargeTime` _output_get (`self.ChargeTime`))
                (bind (_asynctaskproxy _heldtime) (`AbilityTask_ICWaitInputReleased.ICWaitInputReleased` 0.2)
                  (:`OnReleased`
                    (`|ExecutionSequence`
                      (:`then_0`
                        (`AbilitySystemBlueprintLibrary.AddLooseGameplayTags` _returnvalue_6 (`BlueprintGameplayTagLibrary.MakeLiteralGameplayTagContainer` (struct :`GameplayTags` (struct :`(TagName` "State.InCombo")))) true)
                        (`self.MontageStop` -1.0)
                        (`AbilitySystemBlueprintLibrary.RemoveLooseGameplayTags` _returnvalue_6 _returnvalue_5 true)
                        (if (< _heldtime (`self.ChargeTime`))
                          (`AbilityTask_PlayMontageAndWait.CreatePlayMontageAndWaitProxy` "None" "/Game/Character/Assets/Samurai2/ReTargetAnim/Anim/Attack/Montage/Combo1_Attack1_Root_Montage.Combo1_Attack1_Root_Montage" 1.0 (`self.CurrentComboSection`) true 1.0 0.0 true
                            (:`OnCompleted`
                              (set `self.RestartCombo` true :!label _label)
                              (`self.K2_EndAbility`))
                            (:`OnInterrupted`
                              (`self.K2_EndAbility` :!label _label_2))
                            (:`OnCancelled`
                              (goto _label)))
                          (else
                            (`AbilityTask_PlayMontageAndWait.CreatePlayMontageAndWaitProxy` "None" "/Game/Character/Assets/Samurai2/ReTargetAnim/Anim/Attack/Montage/AS_Dash_Air_Attack_Seq_Montage.AS_Dash_Air_Attack_Seq_Montage" 1.0 "None" true 1.0 0.0 true
                              (:`OnCompleted`
                                (goto _label))
                              (:`OnInterrupted`
                                (goto _label_2))
                              (:`OnCancelled`
                                (goto _label))))))
                      (:`then_1`
                        (`/Game/Widgets/WBP/WBP_ChargeBar.ChangeIncrement` _output_get false)
                        (`GameplayTask_WaitDelay.TaskWaitDelay` null 0.5
                          (:`OnFinish`
                            (`Widget.RemoveFromParent` _output_get))))))))))))
      (:`Weapon.Bow`
        (if (`KismetSystemLibrary.IsValid` _returnvalue_8)
          _
          (else
            _))
        (`BowComponent.EnterAimMode` _returnvalue_8)
        (`AbilitySystemBlueprintLibrary.AddLooseGameplayTags` _returnvalue_3 _returnvalue true)
        (bind (_asynctaskproxy_2 _heldtime_2) (`AbilityTask_ICWaitInputReleased.ICWaitInputReleased` 0.2)
          (:`then`
            ; 待机-》拉弓
            (`AbilityTask_PlayMontageAndWait.CreatePlayMontageAndWaitProxy` "None" "/Game/Character/Assets/Samurai2/ReTargetAnim/Anim/Bow/Montage/Bow_Shoot_2_Aim_Montage.Bow_Shoot_2_Aim_Montage"))
          (:`OnReleased`
            (`AbilitySystemBlueprintLibrary.RemoveLooseGameplayTags` _returnvalue_3 _returnvalue true)
            (if (`GameplayTagAssetInterface.HasMatchingGameplayTag` (`self.GetAbilitySystemComponentFromActorInfo`) (struct :`TagName` "State.InDodge"))
              (`self.K2_EndAbility`)
              (else
                (`BowComponent.ExitAimMode` _returnvalue_8)
                (`self.MontageStop` -1.0)
                (`BowComponent.TryLaunchArrow` _returnvalue_8 _heldtime_2)
                (`self.K2_EndAbility`)))))))))

(event `self.K2_OnEndAbility`
  (params (bWasCancelled :type Boolean))
  (bind _returnvalue (`GameplayStatics.GetPlayerController` 0))
  (bind (_value _returnvalue_2) (`BlueprintMapLibrary.Map_Find` (`self.MontageComboMap`) (`self.CurrentComboSection`)))
  (`/Engine/EditorBlueprintResources/StandardMacros.IsValid` _returnvalue
    (:`Is Valid`
      (`Controller.SetIgnoreMoveInput` _returnvalue false)
      (`AbilitySystemBlueprintLibrary.RemoveLooseGameplayTags` (`self.GetOwningActorFromActorInfo`) (`BlueprintGameplayTagLibrary.MakeLiteralGameplayTagContainer` (struct :`GameplayTags` (struct :`(TagName` "State.LockAttack") :`(TagName` "State.InCombo")))))
      (if (`self.RestartCombo`)
        (set `self.CurrentComboSection` "FirstCombo")
        (elif _returnvalue_2
          (set `self.CurrentComboSection` (break `ComboInfo` _value))
          (else
            (set `self.CurrentComboSection` "FirstCombo"))))
      (`self.ResetValue`))))

(fn `ResetValue`
  (bind _wbpcharge (`self.WBPCharge`))
  (set `self.RestartCombo` false)
  (`/Engine/EditorBlueprintResources/StandardMacros.IsValid` _wbpcharge
    (:`Is Valid`
      (`Widget.RemoveFromParent` _wbpcharge))))