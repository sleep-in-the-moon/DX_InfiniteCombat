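; Gameplay ability for enemy attacks, branching on the current weapon's gameplay tag from the avatar's CombatCharacterComponent.
; Staff, sword-shield and hammer each play their own montage, with staff and sword-shield first moving the weapon to its equip socket.
; On staff montage blend-out, it spawns a magic bullet at the weapon socket, launched toward and tracking the player.
; Montage completion, interruption or cancellation clears State.LockAttack and ends the ability.
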(event `self.K2_ActivateAbility`
  (bind _returnvalue (`self.GetOwningActorFromActorInfo`))
  (bind _returnvalue_2 (`GameplayStatics.GetPlayerCharacter` 0))
  (bind _returnvalue_3 (`Actor.GetComponentByClass` (`self.GetAvatarActorFromActorInfo`) "/Script/DX_InfiniteCombat.CombatCharacterComponent"))
  (bind _returnvalue_4 (`SceneComponent.GetSocketLocation` (`CombatCharacterComponent.GetWeaponMeshComponent` (`Actor.GetComponentByClass` (`self.GetAvatarActorFromActorInfo`) "/Script/DX_InfiniteCombat.CombatCharacterComponent")) "BulletLaunchLoc"))
  (bind _returnvalue_5 (`self.K2_CommitAbility`))
  (if _returnvalue_5
    (`/Engine/EditorBlueprintResources/StandardMacros.IsValid` _returnvalue_3
      (:`Is Valid`
        (`|SwitchGameplayTag` (`WeaponDataAsset.WeaponTag` (`CombatCharacterComponent.GetCurrentWeapon` _returnvalue_3))
          (:`Weapon.Staff`
            (`CombatCharacterComponent.CurWeaponToEquipSocket` _returnvalue_3)
            (`AbilityTask_PlayMontageAndWait.CreatePlayMontageAndWaitProxy` "None" "/Game/Character/Assets/SkeletonArmy/Anim/Sorcerer/Montage/AM_skeleton_magic_shot_stright_Montage.AM_skeleton_magic_shot_stright_Montage"
              (:`OnCompleted`
                (`self.MontageEnd` :!label _label))
              (:`OnBlendOut`
                (bind _returnvalue_6 (`|SpawnActorFromClass` "/Game/Weapon/BP/Bullets/BP_MagicBullet.BP_MagicBullet_C" (`KismetMathLibrary.MakeTransform` _returnvalue_4) "Undefined" "MultiplyWithRoot" _returnvalue null))
                (`AbilitySystemBlueprintLibrary.RemoveLooseGameplayTags` _returnvalue (`BlueprintGameplayTagLibrary.MakeLiteralGameplayTagContainer` (struct :`GameplayTags` (struct :`(TagName` "State.LockAttack")))))
                (`ProjectorActorBase.Launch` _returnvalue_6 0.0 (`KismetMathLibrary.Normal` (- (`Actor.K2_GetActorLocation` _returnvalue_2) _returnvalue_4)) 10.0)
                (`ProjectorActorBase.EnableTraceBySocketName` _returnvalue_6 (`|MakeArray` "ObjectTypeQuery1" "ObjectTypeQuery3" "ObjectTypeQuery4" :!type "EObjectTypeQuery Enum") true "DamageLoc")
                (`ProjectorActorBase.TraceObj` _returnvalue_6 _returnvalue_2))
              (:`OnInterrupted`
                (goto _label))
              (:`OnCancelled`
                (goto _label))))
          (:`Weapon.SwordShield`
            (`CombatCharacterComponent.CurWeaponToEquipSocket` _returnvalue_3)
            (`AbilityTask_PlayMontageAndWait.CreatePlayMontageAndWaitProxy` "None" "/Game/Character/Assets/SkeletonArmy/Anim/Footman/AM_Skeleton_1H_swing_left.AM_Skeleton_1H_swing_left"
              (:`OnCompleted`
                _)
              (:`OnInterrupted`
                _)
              (:`OnCancelled`
                _))
            (`self.MontageEnd`))
          (:`Weapon.Hammer`
            (`AbilityTask_PlayMontageAndWait.CreatePlayMontageAndWaitProxy` "None" "/Game/StoneGolem/Animations/AS_StoneGolem_attack4_Montage.AS_StoneGolem_attack4_Montage"
              (:`OnCompleted`
                _)
              (:`OnInterrupted`
                _)
              (:`OnCancelled`
                _))
            (`self.MontageEnd`)))))))

(fn `MontageEnd`
  (`AbilitySystemBlueprintLibrary.RemoveLooseGameplayTags` (`self.GetOwningActorFromActorInfo`) (`BlueprintGameplayTagLibrary.MakeLiteralGameplayTagContainer` (struct :`GameplayTags` (struct :`(TagName` "State.LockAttack")))))
  (`self.K2_EndAbility`))