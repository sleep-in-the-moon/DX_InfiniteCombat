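; GA_GetHurt is a Gameplay Ability named for a character's hurt reaction, but its ActivateAbility event is empty, so it currently does nothing.
; A disconnected chain commits the ability, then plays the CombatCharacterComponent's GetHurtMontage if no montage is already playing.
; That unused chain ends the ability when the montage finishes, is interrupted or is cancelled, and on some failed checks.
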(event `self.K2_ActivateAbility`)