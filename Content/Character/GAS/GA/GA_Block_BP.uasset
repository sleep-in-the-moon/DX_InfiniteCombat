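; Gameplay Ability for blocking that waits for one BlockTrigger event and turns it into a counter.
; On the event it fires camera shake, a clash sound and brief global slow motion.
; It locks onto the instigator via WeakLockComponent and spawns sparks using the AttackEventData payload's hit point.
; It plays CombatCharacterComponent's counter montage, ending on completion; the block-hit montage branch is disconnected.
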(event `self.K2_ActivateAbility`
  (bind _returnvalue (`Actor.GetComponentByClass` (`self.GetAvatarActorFromActorInfo`) "/Script/DX_InfiniteCombat.CombatCharacterComponent"))
  (bind _returnvalue_2 (`Actor.GetComponentByClass` (`self.GetAvatarActorFromActorInfo`) "/Script/DX_InfiniteCombat.WeakLockComponent"))
  (bind ((`BlockHitedMontage` _blockhitedmontage) (`BlockCounterMontage` _blockcountermontage)) (break `BlockMontages` (`CombatCharacterComponent.BlockMontages` _returnvalue)))
  (bind (_asynctaskproxy _payload) (`AbilityTask_WaitGameplayEvent.WaitGameplayEvent` (struct :`TagName` "GameplayEvent.BlockTrigger") null true)
    (:`EventReceived`
      (`|ExecutionSequence`
        (:`then_0`
          (bind _asdx_iccharacter (cast `DX_ICCharacter` (`self.GetAvatarActorFromActorInfo`)))
          (bind _asplayer_controller (cast `PlayerController` (`Pawn.GetController` _asdx_iccharacter)))
          (`PlayerCameraManager.StartCameraShakeFromSource` :`self` (`PlayerController.PlayerCameraManager` _asplayer_controller) :`ShakeClass` "/Game/Character/GAS/GC/CS_Hit.CS_Hit_C"))
        (:`then_1`
          (`GameplayStatics.PlaySoundAtLocation` "/Game/Sounds/Sword/Clash2.Clash2" (`Actor.K2_GetActorLocation` (`self.GetAvatarActorFromActorInfo`)) (struct) 1.0 1.0 0.0 null null null null)
          (`GameplayStatics.SetGlobalTimeDilation` 0.7)
          (`KismetSystemLibrary.RetriggerableDelay` 0.4)
          (`GameplayStatics.SetGlobalTimeDilation` 1.0))
        (:`then_2`
          (`/Engine/EditorBlueprintResources/StandardMacros.IsValid` _returnvalue_2
            (:`Is Valid`
              (bind ((`Instigator` _instigator) (`OptionalObject` _optionalobject)) (break `GameplayEventData` _payload))
              (`/Engine/EditorBlueprintResources/StandardMacros.IsValid` _instigator
                (:`Is Valid`
                  (`WeakLockComponent.SetLockByActor` _returnvalue_2 _instigator)
                  (bind _asattack_event_data (cast `AttackEventData` _optionalobject))
                  (`NiagaraFunctionLibrary.SpawnSystemAtLocation` "/Game/Art/Generic/NS_Spark.NS_Spark" (`AttackEventData.HitLocation` _asattack_event_data) (`KismetMathLibrary.Conv_VectorToRotator` (`AttackEventData.ImpactNormal` _asattack_event_data))))))))
        (:`then_3`
          (`/Engine/EditorBlueprintResources/StandardMacros.IsValid` _returnvalue
            (:`Is Valid`
              (`/Engine/EditorBlueprintResources/StandardMacros.IsValid` _blockcountermontage
                (:`Is Valid`
                  (`AbilityTask_PlayMontageAndWait.CreatePlayMontageAndWaitProxy` "None" _blockcountermontage
                    (:`OnCompleted`
                      (`self.K2_EndAbility`))))))))))))