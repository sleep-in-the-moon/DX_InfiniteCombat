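; Base enemy character Blueprint that handles health bar feedback, execution readiness and death.
; Health changes from the Ability System Component update the StateBar widget and show it until a retriggerable delay hides it.
; The Execute component's state change toggles a red bar border while the enemy can be executed.
; CombatComp's death event flags the AI controller as dead, hides the bar, disables movement and capsule collision, and ragdolls the mesh from the pelvis down.
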(event `DiedEvent`
  (bind _mesh (`self.Mesh`))
  (`|ExecutionSequence`
    (:`then_0`
      (bind _asicaicontroller (cast `ICAIController` (`AIBlueprintHelperLibrary.GetAIController` self)))
      (`ICAIController.UpdateDeadKey` _asicaicontroller true)
      (set `Widget.Visibility` "Collapsed" (`WidgetComponent.GetWidget` (`self.StateBar`))))
    (:`then_1`
      (`CharacterMovementComponent.SetMovementMode` (`self.CharacterMovement`) "MOVE_None" 0)
      (`PrimitiveComponent.SetCollisionEnabled` (`self.CapsuleComponent`) "NoCollision")
      (`PrimitiveComponent.SetCollisionObjectType` _mesh "ECC_PhysicsBody")
      (`PrimitiveComponent.SetCollisionEnabled` _mesh "QueryAndPhysics")
      (`SkeletalMeshComponent.SetAllBodiesBelowSimulatePhysics` _mesh "pelvis" true true)
      (`SkeletalMeshComponent.SetAllBodiesBelowPhysicsBlendWeight` _mesh "pelvis" 1.0 true true))))

(event `self.ReceiveBeginPlay`
  (add `ICAbilitySystemComponent.HelthChangeBPDG` (`self.ASC`) (delegate `HelthChange`))
  (set `Widget.Visibility` "Collapsed" (`WidgetComponent.GetWidget` (`self.StateBar`)))
  (`|ExecutionSequence`
    (:`then_0`
      (add `CombatCharacterComponent.DG_CharacterDied` (`self.CombatComp`) (delegate `DiedEvent`)))
    (:`then_1`
      (add `ExecuteComponent.DG_CanBeExecutedStateChange` (`self.Execute`) (delegate `BeExecutedStateChange`)))))

(event `BeExecutedStateChange`
  (params (NewState :type Boolean))
  (bind _aswbp_progress_bar (cast `/Game/Widgets/WBP/WBP_ProgressBar` (`WidgetComponent.GetWidget` (`self.StateBar`))))
  (if NewState
    (`/Game/Widgets/WBP/WBP_ProgressBar.SetBorder` _aswbp_progress_bar NewState (struct :`R` 1.0 :`A` 1.0))
    (else
      (`/Game/Widgets/WBP/WBP_ProgressBar.SetBorder` :`self` _aswbp_progress_bar))))

(event `HelthChange`
  (params (NewHelth :type "Float (single-precision)"))
  (bind (_bsuccessfullyfoundattribute _returnvalue) (`AbilitySystemBlueprintLibrary.GetFloatAttributeFromAbilitySystemComponent` (`self.ASC`) (struct :`AttributeName` "MaxHP" :`Attribute` "/Script/DX_InfiniteCombat.CharacterAttributeSet:MaxHP" :`AttributeOwner` "/Script/CoreUObject.Class'/Script/DX_InfiniteCombat.CharacterAttributeSet'")))
  (bind _aswbp_progress_bar (cast `/Game/Widgets/WBP/WBP_ProgressBar` (`WidgetComponent.GetWidget` (`self.StateBar`))))
  (if _bsuccessfullyfoundattribute
    (`/Game/Widgets/WBP/WBP_ProgressBar.UpdateBarPercent` _aswbp_progress_bar (/ NewHelth _returnvalue))
    (set `Widget.Visibility` "SelfHitTestInvisible" (`WidgetComponent.GetWidget` (`self.StateBar`)))
    (`KismetSystemLibrary.RetriggerableDelay` 7.0)
    (set `Widget.Visibility` "Collapsed" (`WidgetComponent.GetWidget` (`self.StateBar`)))))

(fn `UserConstructionScript`)